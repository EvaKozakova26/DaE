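; Gate_Pig_BP is an interactable pig gate that the player opens and closes with the Interact input.
; A box overlap enables player 0's input and sets a trigger flag, and leaving the box reverses both.
; Each press toggles the Open state, playing or reversing a timeline that scales an Angle variable into the yaw of the PIGDOORS component.
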(event OnComponentBeginOverlap(Box)
  (params (OverlappedComponent :type Primitive%20Component%20Object%20Reference) (OtherActor :type Actor%20Object%20Reference) (OtherComp :type Primitive%20Component%20Object%20Reference) (OtherBodyIndex :type Integer) (bFromSweep :type Boolean) (SweepResult :type Hit%20Result%20Structure%20%28by%20ref%29))
  ;[1 1 1] Gate Interaction
  (Input|EnableInput (Game|GetPlayerController 0))
  (Variables|Default|SetIsTrigger true))

(event OnComponentEndOverlap(Box)
  (params (OverlappedComponent :type Primitive%20Component%20Object%20Reference) (OtherActor :type Actor%20Object%20Reference) (OtherComp :type Primitive%20Component%20Object%20Reference) (OtherBodyIndex :type Integer))
  ;[1 1 1] Gate Interaction
  (Input|DisableInput (Game|GetPlayerController 0))
  (Variables|Default|SetIsTrigger false))

(event Input|ActionEvents|InputActionInteract
  (params (Key :type Key%20Structure :default "None"))
  ;[1 1 1] Gate Branch
  (:Pressed
    (if (Variables|Default|GetIsTrigger)
      (if (not (Variables|Default|GetOpen))
        (Variables|Default|SetOpen true)
        (bind _newtrack_0 (Timeline|Timeline_0 Play)
          (:Update
            (Transformation|SetRelativeRotation (Variables|Default|GetPIG_DOORS) (Math|Rotator|MakeRotator 0.0 0.0 (* _newtrack_0 (Variables|Default|GetAngle))) false false)))
        (else
          (Variables|Default|SetOpen false)
          (Utilities|FlowControl|Delay 0.0)
          (Timeline|Timeline_0 Reverse))))))

(fn ConstructionScript)