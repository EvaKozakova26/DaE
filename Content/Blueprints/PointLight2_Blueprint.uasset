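; A point light Blueprint that toggles on and off when interacted with from inside its trigger capsule.
; Capsule overlap begin and end events enable or disable input for player 0 and set the IsTrigger flag, without checking which actor overlaps.
; While that flag is set, the Interact action drives a FlipFlop that alternates the light's intensity, switching it off on the first press.
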(event OnComponentBeginOverlap(Capsule)
  (params (OverlappedComponent :type Primitive%20Component%20Object%20Reference) (OtherActor :type Actor%20Object%20Reference) (OtherComp :type Primitive%20Component%20Object%20Reference) (OtherBodyIndex :type Integer) (bFromSweep :type Boolean) (SweepResult :type Hit%20Result%20Structure%20%28by%20ref%29))
  ;[1 1 1] Turn light on/off
  (Input|EnableInput (Game|GetPlayerController 0))
  (Variables|Default|SetIsTrigger true))

(event OnComponentEndOverlap(Capsule)
  (params (OverlappedComponent :type Primitive%20Component%20Object%20Reference) (OtherActor :type Actor%20Object%20Reference) (OtherComp :type Primitive%20Component%20Object%20Reference) (OtherBodyIndex :type Integer))
  ;[1 1 1] Turn light on/off
  (Input|DisableInput (Game|GetPlayerController 0))
  (Variables|Default|SetIsTrigger false))

(event EventBeginPlay)

(event EventTick
  (params (DeltaSeconds :type Float%20%28single-precision%29)))

(event Input|ActionEvents|InputActionInteract
  (params (Key :type Key%20Structure :default "None"))
  (bind _pointlightcomponent (Variables|Default|GetPointLightComponent))
  ;[1 1 1] Turn light on/off
  (:Pressed
    (if (Variables|Default|GetIsTrigger)
      (Utilities|FlowControl|FlipFlop
        (:A
          (Rendering|Components|Light|SetIntensity _pointlightcomponent 0.0))
        (:B
          (Rendering|Components|Light|SetIntensity _pointlightcomponent 8.0))))))

(fn ConstructionScript)